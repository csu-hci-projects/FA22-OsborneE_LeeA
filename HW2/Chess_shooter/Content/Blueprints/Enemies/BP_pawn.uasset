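; BP_pawn is an enemy pawn that continually chases the VR player.
; On BeginPlay it casts the player pawn to VRPawn, stores it and starts the chase event, which ignores its PlayerToChase input and reads player pawn 0 directly.
; Each chase uses AI MoveTo toward a random reachable navigation point around the player's location, then re-triggers itself on success or failure, forming an endless loop without Tick.
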(event `self.ReceiveBeginPlay`
  (bind _asvrpawn (cast `/Game/VRTemplate/Blueprints/VRPawn` (`GameplayStatics.GetPlayerPawn` 0)))
  (bind _output_get (set `self.As VRPawn` _asvrpawn))
  (`self.Chase_player` _output_get))

(event `Chase_player`
  (params (`Player to Chase` :type "/Game/VRTemplate/Blueprints/VRPawn Object Reference"))
  (`|AIMoveTo` self (`NavigationSystemV1.K2_GetRandomReachablePointInRadius` (`self.K2_GetActorLocation` (`GameplayStatics.GetPlayerPawn` 0)) 0.0 null null) null 0.05
    (:`OnSuccess`
      _)
    (:`OnFail`
      _))
  (`self.Chase_player` null))

(fn `UserConstructionScript`)