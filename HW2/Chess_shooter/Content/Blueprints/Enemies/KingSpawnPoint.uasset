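; KingSpawnPoint is an enemy spawn point that spawns King AI pawns at its own location, up to a difficulty-based limit.
; BeginPlay casts to MyGameInstance and sets Limit from its Easy, Medium or Hard flag, printing a failure message if the cast fails.
; Tick runs through a latent Delay, spacing spawns about two seconds apart and incrementing Count until it equals Limit.
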(event `self.ReceiveTick`
  (params (DeltaSeconds :type "Float (single-precision)"))
  (if (not (== (`self.Limit`) (`self.Count`)))
    (`KismetSystemLibrary.Delay` 2.0)
    (`AIBlueprintHelperLibrary.SpawnAIFromClass` "/Game/Blueprints/Enemies/King.King_C" null (`self.K2_GetActorLocation`) (struct) false null)
    (set `self.Count` (+ 1 (`self.Count`)))))

(event `self.ReceiveBeginPlay`
  (bind _asmy_game_instance (cast `/Game/VRTemplate/Blueprints/MyGameInstance` (`GameplayStatics.GetGameInstance`))
    (:`then`
      (if (`/Game/VRTemplate/Blueprints/MyGameInstance.Easy` _asmy_game_instance)
        (set `self.Limit` 1)
        (elif (`/Game/VRTemplate/Blueprints/MyGameInstance.Medium` _asmy_game_instance)
          (set `self.Limit` 2)
          (elif (`/Game/VRTemplate/Blueprints/MyGameInstance.Hard` _asmy_game_instance)
            (set `self.Limit` 3)))))
    (:`CastFailed`
      (`KismetSystemLibrary.PrintString` "Failed"))))

(fn `UserConstructionScript`)