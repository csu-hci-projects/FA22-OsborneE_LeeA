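; King enemy that chases the player's VR pawn and blows up when shot.
; On BeginPlay it casts the player pawn to VRPawn and starts the chase, which uses AIMoveTo toward a random reachable point tightly around the player, then calls ChasePlayer again.
; Overlapping a Projectile plays an explosion sound at world origin, spawns an explosion emitter with no location set, and destroys the King.
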(event `self.ReceiveBeginPlay`
  (bind _asvrpawn (cast `/Game/VRTemplate/Blueprints/VRPawn` (`GameplayStatics.GetPlayerPawn` 0)))
  (bind _output_get (set `self.As VRPawn` _asvrpawn))
  (`self.Chase_player` _output_get))

(event `Chase_player`
  (params (Player_to_Chase :type "/Game/VRTemplate/Blueprints/VRPawn Object Reference"))
  (`|AIMoveTo` self (`NavigationSystemV1.K2_GetRandomReachablePointInRadius` (`self.K2_GetActorLocation` (`GameplayStatics.GetPlayerPawn` 0)) 5.0 null null) null 0.05
    (:`then`
      _)
    (:`OnSuccess`
      _)
    (:`OnFail`
      _))
  (`self.Chase_player` null))

(event `self.ReceiveActorBeginOverlap`
  (params (OtherActor :type "Actor Object Reference"))
  (cast `/Game/VRTemplate/Blueprints/Projectile` OtherActor)
  (`GameplayStatics.PlaySoundAtLocation` "/Game/StarterContent/Audio/Explosion01.Explosion01" (0.0 0.0 0.0) (struct) 1.0 1.0 0.0 null null null null)
  (`GameplayStatics.SpawnEmitterAtLocation` "/Game/StarterContent/Particles/P_Explosion.P_Explosion")
  (`self.K2_DestroyActor`))

(fn `UserConstructionScript`)