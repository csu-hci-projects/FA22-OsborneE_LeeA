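; BP_Ball is a ball actor that tracks its own health and loses it on contact with enemies.
; Hits against a BP_enemy subtract a fixed amount from BallHealth and play a rumble sound at the ball's location.
; Tick creates and adds a new Player_stats widget to the viewport every frame, without reusing an earlier one.
; GetBallRef returns the ball itself, while GetBallRef2 is an empty stub.
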(event `self.ReceiveTick`
  (params (DeltaSeconds :type "Float (single-precision)"))
  ;[1 1 1] Health and Lives Wiget
  (bind _returnvalue (`|CreateWidget` "/Game/UI/Player_stats.Player_stats_C"))
  (`UserWidget.AddToViewport` _returnvalue 0))

(event `self.ReceiveActorBeginOverlap`
  (params (OtherActor :type "Actor Object Reference")))

(event `self.ReceiveBeginPlay`)

(event `self.ReceiveHit`
  (params (MyComp :type "PrimitiveComponent Object Reference") (Other :type "Actor Object Reference") (OtherComp :type "PrimitiveComponent Object Reference") (bSelfMoved :type Boolean) (HitLocation :type "Vector Structure") (HitNormal :type "Vector Structure") (NormalImpulse :type "Vector Structure") (Hit :type "HitResult Structure (by ref)"))
  (cast `/Game/Blueprints/BP_enemy` Other)
  (set `self.BallHealth` (- (`self.BallHealth`) 20))
  (`GameplayStatics.PlaySoundAtLocation` "/Game/SuperGrid/TutorialLevel/SoundEffects/Cinematic_deep_rumble.Cinematic_deep_rumble" (`self.K2_GetActorLocation`) (struct) 1.0 1.0 0.0 null null null null))

(fn `GetBallRef`
  (returns (Ball :type "/Game/Blueprints/BP_Ball Object Reference"))
  (return self))

(fn `GetBallRef2`
  (returns (BPBall2 :type "/Game/Blueprints/BP_Ball Object Reference"))
  (return null))

(fn `UserConstructionScript`)