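; CubeBlock is a moving block actor that travels back and forth along a configurable direction.
; A looping timer started on BeginPlay negates Direction every TimeToChange seconds.
; Each Tick offsets the actor along the normalized Direction, scaled by Speed and world delta seconds, without sweeping, so movement ignores collision.
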(event `self.ReceiveBeginPlay`
  (`KismetSystemLibrary.K2_SetTimerDelegate` (delegate `ChangeDirection`) (`self.timeToChange`) true))

(event `ChangeDirection`
  (set `self.Direction` (* (`self.Direction`) -1.0)))

(event `self.ReceiveTick`
  (params (DeltaSeconds :type "Float (single-precision)"))
  (`self.K2_AddActorWorldOffset` (* (`KismetMathLibrary.Normal` (`self.Direction`)) (* (`self.speed`) (`GameplayStatics.GetWorldDeltaSeconds`)))))

(fn `UserConstructionScript`)